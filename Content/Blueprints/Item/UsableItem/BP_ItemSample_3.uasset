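; Sample usable item actor (BP_ItemSample_3) that highlights its cube while the player is near.
; BeginPlay sets the cube to block Visibility traces with query and physics collision and turns custom depth off.
; OverlapCollision begin and end events toggle the cube's custom depth render, identifying the player by the first actor tag "Player".
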(event OnComponentBeginOverlap(OverlapCollision)
  (params (OverlappedComponent :type Primitive%20Component%20Object%20Reference) (OtherActor :type Actor%20Object%20Reference) (OtherComp :type Primitive%20Component%20Object%20Reference) (OtherBodyIndex :type Integer) (bFromSweep :type Boolean) (SweepResult :type Hit%20Result%20Structure%20%28by%20ref%29))
  (if (Utilities|Name|Equal(Name) (Utilities|Array|Get(acopy) (Variables|/Script/Engine.Actor|GetTags OtherActor)) "Player")
    (Rendering|SetRenderCustomDepth (Variables|Default|GetCube) true)))

(event OnComponentEndOverlap(OverlapCollision)
  (params (OverlappedComponent :type Primitive%20Component%20Object%20Reference) (OtherActor :type Actor%20Object%20Reference) (OtherComp :type Primitive%20Component%20Object%20Reference) (OtherBodyIndex :type Integer))
  (if (Utilities|Name|Equal(Name) (Utilities|Array|Get(acopy) (Variables|/Script/Engine.Actor|GetTags OtherActor)) "Player")
    (Rendering|SetRenderCustomDepth (Variables|Default|GetCube) false)))

(event EventBeginPlay
  (bind _cube (Variables|Default|GetCube))
  (Collision|SetCollisionEnabled _cube "QueryAndPhysics")
  (Collision|SetCollisionResponsetoChannel _cube "ECC_Visibility" "ECR_Block")
  (Rendering|SetRenderCustomDepth _cube false))

(event Collision|EventActorBeginOverlap
  (params (OtherActor :type Actor%20Object%20Reference)))

(event EventTick
  (params (DeltaSeconds :type Float%20%28single-precision%29)))

(fn ConstructionScript)